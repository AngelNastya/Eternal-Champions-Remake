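; Stats component that tracks health, stamina and power, firing an event dispatcher when each is depleted.
; Change functions cap health and power at their maximums and manage their empty flags.
; While health remains, Tick moves stamina toward 0 or 100 at a constant rate, as toggled by UseStamina.
; Health regeneration and debug display are stubs with unconnected logic, so nothing regenerates health on Tick.
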(event EventTick
  (params (DeltaSeconds :type Float%20%28single-precision%29))
  (if (not (Variables|Health|GetNo%20Health))
    (CallFunction|CalculateStamina (Variables|Stamina|GetStamina%20Use))
    (else
      (CallFunction|HealthRegeneration))))

(fn ChangeHealth
  (params (Value :type Float%20%28single-precision%29))
  (bind _output_get (Variables|Health|SetHealth (Math|Float|Min(Float) (+ Value (Variables|Health|GetHealth)) (Variables|Health|GetMax%20Health))))
  (if (and (<= _output_get 0.0) (not (Variables|Health|GetNo%20Health)))
    (Variables|Health|SetNo%20Health true)
    (Default|CallHealthEnd)
    (else
      (Variables|Health|SetNo%20Health false))))

(fn DisplayStats)

(fn HealthRegeneration)

(fn CalculateStamina
  (params (Use :type Boolean))
  (bind _output_get (Variables|Stamina|SetStamina (Math|Interpolation|FInterptoConstant (Variables|Stamina|GetStamina) (Math|Float|SelectFloat 0.0 1e+02 Use) (Utilities|Time|GetWorldDeltaSeconds) (Variables|Stamina|GetStamina%20Speed))))
  (if (and (<= _output_get 0.0) (not (Variables|Stamina|GetStaminaEnded)))
    (Variables|Stamina|SetStaminaEnded true)
    (Default|CallStaminaEnd)))

(fn UseStamina
  (params (Use :type Boolean) (UseSpeed :type Float%20%28single-precision%29))
  (bind _output_get (Variables|Stamina|SetStamina%20Use Use))
  (if _output_get
    (Variables|Stamina|SetStamina%20Speed UseSpeed)
    (else
      (Variables|Stamina|SetStaminaEnded false))))

(fn ChangePower
  (params (Power :type Float%20%28single-precision%29))
  (bind _output_get (Variables|Power|SetPower (Math|Float|Min(Float) (+ Power (Variables|Power|GetPower)) (Variables|Power|GetMax%20Power))))
  (if (and (<= _output_get 0.0) (not (Variables|Power|GetNo%20Power)))
    (Variables|Power|SetNo%20Power true)
    (Default|CallPowerEnd)
    (else
      (Variables|Power|SetNo%20Power false))))